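; Explosive barrel actor that detonates once on OnHit, fracturing its mesh with radius damage, playing explosion effects and sound, and firing a radial force impulse.
; Damage to others comes from a Sphere whose collision switches on for 0.1 seconds, sending zombie-hit and generic hit messages to overlapped actors.
; The barrel destroys itself five seconds later.
; Radial-damage and helper-actor spawn nodes are left unconnected.
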(event OnComponentBeginOverlap(Sphere)
  (params (OverlappedComponent :type Primitive%20Component%20Object%20Reference) (OtherActor :type Actor%20Object%20Reference) (OtherComp :type Primitive%20Component%20Object%20Reference) (OtherBodyIndex :type Integer) (bFromSweep :type Boolean) (SweepResult :type Hit%20Result%20Structure%20%28by%20ref%29))
  (Class|BIZombieHit|OnZombieHit(Message) OtherActor (Transformation|GetWorldLocation (Variables|Default|GetSM_Barrel01_DM)) "0, 0, 0" 100)
  (Class|BIHittable|OnHit(Message) OtherActor))

(event EventBeginPlay
  (Collision|SetCollisionProfileName (Variables|Default|GetSphere) "NoCollision" true :!class /Script/Engine.PrimitiveComponent))

(event EventOnHit
  (bind _sm_barrel01_dm (Variables|Default|GetSM_Barrel01_DM))
  (bind _returnvalue (Transformation|GetWorldLocation _sm_barrel01_dm))
  (Utilities|FlowControl|DoOnce false
    (:Completed
      (Effects|SpawnEmitteratLocation "/Game/Assets/Import/Realistic_Starter_VFX_Pack_Vol2/Particles/Explosion/P_Explosion_Big_A.P_Explosion_Big_A" _returnvalue "0, 0, 0" "4.000000,4.000000,4.000000")
      (Class|DestructibleComponent|ApplyRadiusDamage (Variables|Default|GetSM_Barrel01_DM) 1.0 _returnvalue 2e+02 1e+04 true)
      (Audio|PlaySoundatLocation "/Game/StarterContent/Audio/Explosion_Cue.Explosion_Cue" _returnvalue "0, 0, 0" 1.0 1.0 0.0 0 0 0)
      (Class|RadialForceComponent|FireImpulse (Variables|Default|GetRadialForce))
      (Collision|SetCollisionProfileName (Variables|Default|GetSphere) "OverlapAllDynamic" true :!class /Script/Engine.PrimitiveComponent)
      (Utilities|FlowControl|Delay 0.1)
      (Collision|SetCollisionProfileName (Variables|Default|GetSphere) "NoCollision" true :!class /Script/Engine.PrimitiveComponent)
      (Utilities|FlowControl|Delay 5.0)
      (Actor|DestroyActor))))

(fn ConstructionScript)