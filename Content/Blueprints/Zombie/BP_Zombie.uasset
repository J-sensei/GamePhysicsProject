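; Zombie character with limbs that break off when hit.
; The construction script slaves four limb meshes to the body's pose; hits select a part by nearest socket, then detach it into physics with a blood burst.
; Losing a leg sets a crawling flag and crawl-idle animation on the limb meshes.
; The crawl-to-player AI move and detached-part cleanup are unwired; a helper returns normalized speed.
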(event Custom|DetachBodyPart
  (params (HitZombiePart :type Skeletal%20Mesh%20Component%20Object%20Reference))
  (Class|SkinnedMeshComponent|SetMasterPoseComponent HitZombiePart 0 false)
  (Utilities|FlowControl|Delay 0.1)
  (Physics|SetSimulatePhysics HitZombiePart true)
  (Utilities|FlowControl|Sequence
    (:then_0
      (if (and (or (== HitZombiePart (Variables|Default|GetZombie1_LeftLeg)) (== HitZombiePart (Variables|Default|GetZombie1_RightLeg))) (not (Variables|Default|GetCrawling)))
        (Variables|Default|SetCrawling true)
        (Components|Animation|SetAnimation (Variables|Default|GetZombie1_LeftLeg) "/Game/Assets/Import/Zombies/Animations/AS_Zombie_Crawl_Idle.AS_Zombie_Crawl_Idle")))))

(event Custom|CrawToPlayer
  (Utilities|FlowControl|DoOnce false
    (:Completed
      (AI|AIMoveTo self "0, 0, 0" (Game|GetPlayerCharacter 0) 5e+01 false :!label _label
        (:OnSuccess
          (Utilities|FlowControl|Delay 1.0)
          (goto _label))))))

(event EventBeginPlay)

(event Collision|EventActorBeginOverlap
  (params (OtherActor :type Actor%20Object%20Reference)))

(event EventTick
  (params (DeltaSeconds :type Float%20%28single-precision%29)))

(event EventOnZombieHit
  (params (HitLocation :type Vector :default "0, 0, 0") (HitNormal :type Vector :default "0, 0, 0"))
  (bind _hitzombiepart (CallFunction|GetHitZombiePart HitLocation))
  (Development|PrintString (Utilities|GetDisplayName _hitzombiepart))
  (if (and (!= _hitzombiepart (Variables|Character|GetMesh)) (not (Physics|IsSimulatingPhysics _hitzombiepart "None")))
    (CallFunction|DetachBodyPart _hitzombiepart)
    (Effects|SpawnEmitteratLocation "/Game/Assets/Import/Realistic_Starter_VFX_Pack_Vol2/Particles/Blood/P_Blood_Splat_Cone.P_Blood_Splat_Cone" HitLocation)))

(fn ConstructionScript
  (Class|SkinnedMeshComponent|SetMasterPoseComponent (Variables|Default|GetZombie1_LeftLeg) (Variables|Character|GetMesh) false))

(fn GetHitZombiePart
  (params (HitLocation :type Vector))
  (for (_array_element _array_index) (Variables|Default|GetSocketNames)
    (if (< (Math|Vector|Distance(Vector) HitLocation (Transformation|GetSocketLocation (Variables|Character|GetMesh) _array_element)) (LocalVariables|GetClosestDistance))
      (LocalVariables|SetClosestDistance (Math|Vector|Distance(Vector) HitLocation (Transformation|GetSocketLocation (Variables|Character|GetMesh) _array_element)))
      (LocalVariables|SetClosestSocketIndex _array_index)))
  (return (Utilities|Select :Index (LocalVariables|GetClosestSocketIndex) :Option%200 (Variables|Default|GetZombie1_LeftHand) :Option%201 (Variables|Default|GetZombie1_RightHand) :Option%202 (Variables|Default|GetZombie1_LeftLeg) :Option%203 (Variables|Default|GetZombie1_RightLeg) :Option%204 (Variables|Character|GetMesh))))

(fn GetVelocty01
  (return (/ (Math|Vector|VectorLength (Transformation|GetVelocity self)) (Variables|/Script/Engine.CharacterMovementComponent|GetMaxWalkSpeed (Variables|Character|GetCharacterMovement)))))