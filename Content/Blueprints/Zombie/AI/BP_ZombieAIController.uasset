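; BP_ZombieAIController is the zombie AI controller, which runs BT_Zombie with the BB_Zombie blackboard from BeginPlay.
; Its AI perception updates write the sensing result to the SpottedPlayer blackboard key when the actor casts to BP_FirstPersonController.
; Each such update, whether gained or lost, also has a random chance to play a zombie howl at the perceived actor's location, not the zombie's.
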(event OnTargetPerceptionUpdated(AIPerception)
  (params (Actor :type Actor%20Object%20Reference) (Stimulus :type AI%20Stimulus%20Structure))
  (Variables|Default|SetSensed (.bSuccessfullySensed (Utilities|Struct|BreakAIStimulus Stimulus)))
  (Utilities|Casting|CastToBP_FirstPersonController Actor)
  (AI|Components|Blackboard|SetValueasBool (AI|GetBlackboard 0) (Utilities|Name|MakeLiteralName "SpottedPlayer") (Variables|Default|GetSensed))
  (if (Math|Random|RandomBool)
    (Audio|PlaySoundatLocation "/Game/Assets/Audio/Zombie/Zombie_Howl_Cue.Zombie_Howl_Cue" (Transformation|GetActorLocation Actor) "0, 0, 0" 1.0 1.0 0.0 "/Game/Assets/Audio/Footsteps/FootstepAttenuation.FootstepAttenuation" 0 0)))

(event EventBeginPlay
  ;[1 1 1] Set Bajavior Tree
  (AI|RunBehaviorTree "/Game/Blueprints/Zombie/AI/BT_Zombie.BT_Zombie")
  (Class|AIController|UseBlackboard "/Game/Blueprints/Zombie/AI/BB_Zombie.BB_Zombie"))

(event EventTick
  (params (DeltaSeconds :type Float%20%28single-precision%29)))

(fn ConstructionScript)