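; BP_Zombie2 is a zombie enemy variant that only configures values on a parent Blueprint, with no gameplay logic of its own.
; Its construction script runs the parent's, then sets the animation set for crawling, attacks and neck bite, along with health, damage, movement speeds and score.
; It also sets an ammo pickup as its possible drop with a drop rate.
; The event graph holds only disabled placeholder events.
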(event EventBeginPlay
  (|CallParentFunction) ; This node is disabled and will not be called.\nDrag off pins to build functionality.
)

(event Collision|EventActorBeginOverlap
  (params (OtherActor :type Actor%20Object%20Reference)))

(event EventTick
  (params (DeltaSeconds :type Float%20%28single-precision%29)))

(fn ConstructionScript
  (|CallParentFunction)
  (Variables|Default|SetAnimationData (Utilities|Struct|MakeF_ZombieAnimation "/Game/Assets/Import/Zombies/Zombie2/Animation/AS_Zombie2_Crawl_Idle.AS_Zombie2_Crawl_Idle" "/Game/Assets/Import/Zombies/Zombie2/Animation/AS_Zombie2_Crawl_Death.AS_Zombie2_Crawl_Death" "/Game/Assets/Import/Zombies/Zombie2/Animation/AS_Zombie2_Attack1_Montage.AS_Zombie2_Attack1_Montage" "/Game/Assets/Import/Zombies/Zombie2/Animation/AS_Zombie2_Attack2_Montage.AS_Zombie2_Attack2_Montage" "/Game/Assets/Import/Zombies/Zombie2/Animation/AS_Zombie2_Neck_Bite_Montage.AS_Zombie2_Neck_Bite_Montage" "/Game/Assets/Import/Zombies/Zombie2/Animation/AS_Zombie2_Crawl_Attack_Montage.AS_Zombie2_Crawl_Attack_Montage"))
  (Variables|Default|SetHP 5)
  (Variables|Default|SetAttackDamage 6.0)
  (Variables|Default|SetMaxSpeed 3.5e+02)
  (Variables|Default|SetCrawlSpeed 125.0)
  (Variables|Default|SetWanderSpeedMultiplier 0.25)
  (Variables|Default|SetChaseSpeedMultiplier 1.0)
  (Variables|Default|SetPickupSpawnList (Utilities|Array|MakeArray "/Game/Blueprints/Pickup/BP_PickupAmmo.BP_PickupAmmo_C"))
  (Variables|Default|SetDropRate 0.2)
  (Variables|Default|SetScore 12))