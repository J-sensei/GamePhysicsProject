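; Base zombie character with dismemberment, melee attacks and death handling, which despawns when far from the player.
; Hits map to the nearest socket's body part, detaching it from the master pose into physics; head loss kills, leg loss triggers crawling.
; Attack montages depend on crawling and remaining hands, applying damage on notify if in range.
; Death ragdolls or plays a crawl animation, notifies listeners, awards score and may drop a pickup.
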(event Custom|DetachBodyPart
  (params (HitZombiePart :type Skeletal%20Mesh%20Component%20Object%20Reference))
  ;[1 1 1] Detach Body Part
  (Class|SkinnedMeshComponent|SetMasterPoseComponent HitZombiePart 0 false)
  (Utilities|FlowControl|Delay 0.1)
  (Physics|SetSimulatePhysics HitZombiePart true)
  (Utilities|FlowControl|Sequence
    (:then_0
      ;;[1 1 1] Set to crawling
      (if (and (or (== HitZombiePart (Variables|Default|GetZombie1_LeftLeg)) (== HitZombiePart (Variables|Default|GetZombie1_RightLeg))) (not (Variables|Default|GetCrawling)))
        (Variables|Default|SetCrawling true)
        (Components|Animation|SetAnimation (Variables|Default|GetZombie1_LeftLeg) (Utilities|Struct|BreakF_ZombieAnimation (Variables|Data|GetAnimationData)))
        (Variables|Movement|SetMaxSpeed (Variables|Movement|GetCrawlSpeed))))))

(event Custom|Attack
  (bind _animationdata (Variables|Data|GetAnimationData))
  (bind _animationdata_2 (Variables|Data|GetAnimationData))
  (bind _attackdelaydata (Variables|Data|GetAttackDelayData))
  (bind (_crawlidle _attack1 _attack2) (Utilities|Struct|BreakF_ZombieAnimation _animationdata))
  (bind (_crawlidle_2 _attack2_2 _neckbite) (Utilities|Struct|BreakF_ZombieAnimation _animationdata_2))
  (bind (_attack1_2 _attack2_3) (Utilities|Struct|BreakF_ZombieAttackDelay _attackdelaydata))
  ;[1 0 0] Zombie Attack
  (if (Variables|Default|GetCrawling)
    ;;[1 1 1] Crawl Attack
    (Animation|Montage|PlayMontage (Variables|Character|GetMesh) (.CrawlAttack (Utilities|Struct|BreakF_ZombieAnimation (Variables|Data|GetAnimationData)))
      (:then
        (Variables|Default|SetAttackDelay (Utilities|Struct|BreakF_ZombieAttackDelay (Variables|Data|GetAttackDelayData))))
      (:OnNotifyBegin
        (CallFunction|OnAttack :!label _label)))
    (elif (Physics|IsSimulatingPhysics (Variables|Default|GetZombie1_RightHand) "None")
      (if (Physics|IsSimulatingPhysics (Variables|Default|GetZombie1_LeftHand) "None")
        ;;[1 1 1] Lost both hand, only can bite
        (Animation|Montage|PlayMontage (Variables|Character|GetMesh) _neckbite
          (:then
            (Variables|Default|SetAttackDelay (Utilities|Struct|BreakF_ZombieAttackDelay (Variables|Data|GetAttackDelayData))))
          (:OnNotifyBegin
            (goto _label)))
        (else
          ;;[1 1 1] Attack with left arm is blow off
          (Animation|Montage|PlayMontage (Variables|Character|GetMesh) _attack2_2
            (:then
              (Variables|Default|SetAttackDelay (Utilities|Struct|BreakF_ZombieAttackDelay (Variables|Data|GetAttackDelayData))))
            (:OnNotifyBegin
              (goto _label)))))
      (else
        ;;[1 1 1] Attack when both hand exist
        (if (Math|Random|RandomBool)
          (Animation|Montage|PlayMontage (Variables|Character|GetMesh) _attack1
            (:then
              (Variables|Default|SetAttackDelay _attack1_2))
            (:OnNotifyBegin
              (goto _label)))
          (else
            (Animation|Montage|PlayMontage (Variables|Character|GetMesh) _attack2
              (:then
                (Variables|Default|SetAttackDelay _attack2_3))
              (:OnNotifyBegin
                (goto _label)))))))))

(event Custom|Kill
  (params (HitLocation :type Vector) (HitNormal :type Vector))
  (bind _mesh (Variables|Character|GetMesh))
  (bind _pickupspawnlist (Variables|Pickup|GetPickupSpawnList))
  ;[1 0.2352 0.1814] Kill the zombie
  (AI|Logic|StopLogic (Variables|/Script/AIModule.AIController|GetBrainComponent (AI|GetAIController self)) "Zombie HP drops to 0")
  (Components|Movement|StopMovementImmediately (Variables|Character|GetCharacterMovement))
  (if (Variables|Default|GetCrawling)
    (Components|Animation|PlayAnimation (Variables|Character|GetMesh) (.CrawlDeath (Utilities|Struct|BreakF_ZombieAnimation (Variables|Data|GetAnimationData))) false)
    (else
      (Collision|SetCollisionProfileName _mesh "Ragdoll" true :!class /Script/Engine.PrimitiveComponent)
      (Physics|SetSimulatePhysics _mesh true)
      (Collision|SetCollisionProfileName (Variables|Collision|GetCapsuleComponent) "NoCollision" true :!class /Script/Engine.PrimitiveComponent)
      (bind _result (Math|Float|NegateFloat (Variables|Default|GetImpulseForce))
        (:%20%20
          (Physics|AddImpulseatLocation (Variables|Character|GetMesh) (* HitNormal _result) HitLocation "None")))))
  (Utilities|FlowControl|Sequence
    (:then_0
      ;;[1 1 1] Inform other listeners this zombie is killed
      (Default|CallOnZombieKill self)
      (Utilities|FlowControl|Delay 5.0)
      (Actor|DestroyActor))
    (:then_1
      (if (and (< (Math|Random|RandomFloatinRange 0.0 1.0) (Variables|Pickup|GetDropRate)) (> (Utilities|Array|Length _pickupspawnlist) 0))
        (Utilities|FlowControl|DoOnce false
          (:Completed
            (Game|SpawnActorfromClass (.OutItem (Utilities|Array|Random _pickupspawnlist)) (Math|Transform|MakeTransform (Transformation|GetActorLocation) "0, 0, 0" "1,1,1") "Undefined" 0 0)))))
    (:then_2
      (Utilities|FlowControl|DoOnce false
        (:Completed
          (Class|BIScore|AddScore(Message) (Game|GetPlayerCharacter 0) (Variables|Default|GetScore) (Variables|Default|GetHeadshot)))))
    (:then_3
      (Audio|PlaySoundatLocation "/Game/Assets/Audio/Zombie/Death/Zombie_Death_Cue.Zombie_Death_Cue" (Transformation|GetActorLocation) "0, 0, 0" 1.0 1.0 0.0 "/Game/Assets/Audio/Footsteps/FootstepAttenuation.FootstepAttenuation" 0 0))))

(event Custom|OnAttack
  (bind _returnvalue (Math|Random|RandomFloatinRange 0.7 1.2))
  (bind _returnvalue_2 (Game|GetPlayerCharacter 0))
  (bind _returnvalue_3 (+ _returnvalue 1.0))
  ;[1 0.1369 0.09913] When zombie attacked the player
  (if (> (Variables|Default|GetHP) 0)
    (if (<= (Transformation|GetDistanceTo _returnvalue_2 self) (Variables|Default|GetAttackRange))
      (Class|BIPlayerDamage|OnPlayerHit(Message) (.AsBP%20First%20Person%20Controller (Utilities|Casting|CastToBP_FirstPersonController _returnvalue_2)) (Variables|Default|GetAttackDamage) (Transformation|GetActorLocation))
      (Audio|PlaySoundatLocation "/Game/Assets/Audio/HitSound/ZombieHit_Cue.ZombieHit_Cue" "0, 0, 0" "0, 0, 0" _returnvalue_3 _returnvalue_3 0.0 0 0 0)
      (Camera|PlayWorldCameraShake "/Game/Blueprints/Interactable/BP_ExplosiveShake.BP_ExplosiveShake_C" (Transformation|GetActorLocation) 0.0 5e+02))))

(event Custom|DeleteZombie
  ;[1 0.8299 0.2351] Delete Zombie
  ;;[1 1 1] Inform other listeners this zombie is killed
  (Default|CallOnZombieKill self)
  (Actor|DestroyActor))

(event Custom|CheckZombieDestroy
  ;[1 1 1] Destroy zombie if too far away from the player
  (if (>= (Class|KismetMathLibrary|VectorDistanceSquared (Transformation|GetActorLocation (Game|GetPlayerCharacter 0)) (Transformation|GetActorLocation self)) (Math|Float|Square (Variables|Default|GetDestroyDistance)))
    (CallFunction|DeleteZombie)))

(event Custom|BloodCollide
  (params (EventName :type Name) (EmitterTime :type Float%20%28single-precision%29) (ParticleTime :type Integer) (Location :type Vector) (Velocity :type Vector) (Direction :type Vector) (Normal :type Vector) (BoneName :type Name) (PhysMat :type Physical%20Material%20Object%20Reference))
  (Rendering|Decal|SpawnDecalatLocation "/Game/Assets/Materials/Blood/M_BloodDecal.M_BloodDecal" (Math|Conversions|ToVector(Float) (Math|Random|RandomFloatinRange 2e+01 3e+01)) Location (Math|Conversions|RotationFromXVector Normal) 1e+01))

(event EventBeginPlay
  (bind _returnvalue (Math|Random|RandomFloatinRange 0.9 1.1))
  (Transformation|SetWorldScale3D (Variables|Collision|GetCapsuleComponent) (Math|Vector|MakeVector _returnvalue _returnvalue _returnvalue))
  (Transformation|SetActorRotation (Math|Rotator|MakeRotator 0.0 0.0 (Math|Random|RandomFloatinRange 0.0 3.6e+02)))
  (Variables|/Script/Engine.CharacterMovementComponent|SetMaxWalkSpeed (Variables|Character|GetCharacterMovement) (Variables|Movement|GetMaxSpeed))
  (Utilities|Time|SetTimerbyEvent (delegate Custom|CheckZombieDestroy) 0.5 true))

(event EventOnZombieHit
  (params (HitLocation :type Vector :default "0, 0, 0") (HitNormal :type Vector :default "0, 0, 0") (Damage :type Integer))
  (bind _hitzombiepart (CallFunction|GetHitZombiePart HitLocation))
  (Utilities|FlowControl|Sequence
    (:then_0
      (if (and (!= _hitzombiepart (Variables|Character|GetMesh)) (not (Physics|IsSimulatingPhysics _hitzombiepart "None")))
        (CallFunction|DetachBodyPart _hitzombiepart)
        (if (== _hitzombiepart (Variables|Default|GetZombie1_Head))
          (Variables|Default|SetHP 0)
          (Variables|Default|SetHeadshot true))))
    (:then_1
      ;[1 1 1] Deduct HP
      (bind _output_get (Variables|Default|SetHP (- (Variables|Default|GetHP) Damage)))
      (if (<= _output_get 0)
        (CallFunction|Kill HitLocation HitNormal)
        (Rendering|Decal|SpawnDecalatLocation "/Game/Assets/Materials/Blood/M_BloodDecal.M_BloodDecal" (Math|Conversions|ToVector(Float) (Math|Random|RandomFloatinRange 2e+01 3e+01)) HitLocation (Math|Conversions|RotationFromXVector HitNormal) 1e+01)))
    (:then_3
      (bind _returnvalue (Effects|SpawnEmitteratLocation "/Game/Assets/Import/Realistic_Starter_VFX_Pack_Vol2/Particles/Blood/P_Blood_Splat_Cone.P_Blood_Splat_Cone" HitLocation (Math|Rotator|MakeRotfromX HitNormal) "1.500000,1.500000,1.500000"))
      (EventDispatchers|BindEventtoOnParticleCollide _returnvalue (delegate Custom|BloodCollide)))))

(fn ConstructionScript
  (Class|SkinnedMeshComponent|SetMasterPoseComponent (Variables|Default|GetZombie1_LeftLeg) (Variables|Character|GetMesh) false))

(fn GetHitZombiePart
  (params (HitLocation :type Vector))
  (for (_array_element _array_index) (Variables|Default|GetSocketNames)
    (if (< (Math|Vector|Distance(Vector) HitLocation (Transformation|GetSocketLocation (Variables|Character|GetMesh) _array_element)) (LocalVariables|GetClosestDistance))
      (LocalVariables|SetClosestDistance (Math|Vector|Distance(Vector) HitLocation (Transformation|GetSocketLocation (Variables|Character|GetMesh) _array_element)))
      (LocalVariables|SetClosestSocketIndex _array_index)))
  (return (Utilities|Select :Index (LocalVariables|GetClosestSocketIndex) :Option%200 (Variables|Default|GetZombie1_LeftHand) :Option%201 (Variables|Default|GetZombie1_RightHand) :Option%202 (Variables|Default|GetZombie1_LeftLeg) :Option%203 (Variables|Default|GetZombie1_RightLeg) :Option%204 (Variables|Default|GetZombie1_Head) :Option%205 (Variables|Character|GetMesh))))

(fn GetVelocty01
  (return (/ (Math|Vector|VectorLength (Transformation|GetVelocity self)) (Variables|Movement|GetMaxSpeed))))