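; BP_Zombie3 is a zombie enemy variant that inherits its behavior from a parent Blueprint and adds no active event logic of its own.
; Its construction script runs the parent's, then sets the variant's crawl, attack, neck bite and death animations.
; The same script overrides health, damage, movement speeds, attack range, score, destroy distance, and ammo or big medkit drops with their drop rate.
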(event EventBeginPlay
  (|CallParentFunction) ; This node is disabled and will not be called.\nDrag off pins to build functionality.
)

(event Collision|EventActorBeginOverlap
  (params (OtherActor :type Actor%20Object%20Reference)))

(event EventTick
  (params (DeltaSeconds :type Float%20%28single-precision%29)))

(fn ConstructionScript
  (|CallParentFunction)
  (Variables|Default|SetAnimationData (Utilities|Struct|MakeF_ZombieAnimation "/Game/Assets/Import/Zombies/Zombie3/Animation/AS_Zombie3_Crawl_Idle.AS_Zombie3_Crawl_Idle" "/Game/Assets/Import/Zombies/Zombie3/Animation/AS_Zombie3_Crawl_Death.AS_Zombie3_Crawl_Death" "/Game/Assets/Import/Zombies/Zombie3/Animation/AS_Zombie3_Attack1_Montage.AS_Zombie3_Attack1_Montage" "/Game/Assets/Import/Zombies/Zombie3/Animation/AS_Zombie3_Attack2_Montage.AS_Zombie3_Attack2_Montage" "/Game/Assets/Import/Zombies/Zombie3/Animation/AS_Zombie3_Neck_Bite_Montage.AS_Zombie3_Neck_Bite_Montage" "/Game/Assets/Import/Zombies/Zombie3/Animation/AS_Zombie3_Crawl_Attack_Montage.AS_Zombie3_Crawl_Attack_Montage"))
  (Variables|Default|SetHP 8)
  (Variables|Default|SetAttackDamage 1e+01)
  (Variables|Default|SetMaxSpeed 6e+02)
  (Variables|Default|SetCrawlSpeed 4e+02)
  (Variables|Default|SetWanderSpeedMultiplier 0.5)
  (Variables|Default|SetChaseSpeedMultiplier 1.0)
  (Variables|Default|SetPickupSpawnList (Utilities|Array|MakeArray "/Game/Blueprints/Pickup/BP_PickupAmmo.BP_PickupAmmo_C" "/Game/Blueprints/Pickup/BP_PickupBigMedkit.BP_PickupBigMedkit_C"))
  (Variables|Default|SetDropRate 0.8)
  (Variables|Default|SetScore 20)
  (Variables|Default|SetAttackRange 2e+02)
  (Variables|Default|SetDestroyDistance 4.5e+03))