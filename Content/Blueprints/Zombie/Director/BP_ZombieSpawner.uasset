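; Trigger-volume zombie spawner that asks for a group of zombies when the player walks into it.
; A BP_FirstPersonController overlapping TriggerBox fires the RequestZombieSpawn dispatcher with a random count in the min/max range and the SpawnPoint location, leaving the actual spawning to listeners.
; Each activation switches the box's collision off and a timer restores it after a 30-second cooldown.
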(event OnComponentBeginOverlap(TriggerBox)
  (params (OverlappedComponent :type Primitive%20Component%20Object%20Reference) (OtherActor :type Actor%20Object%20Reference) (OtherComp :type Primitive%20Component%20Object%20Reference) (OtherBodyIndex :type Integer) (bFromSweep :type Boolean) (SweepResult :type Hit%20Result%20Structure%20%28by%20ref%29))
  (Utilities|Casting|CastToBP_FirstPersonController OtherActor)
  (Collision|SetCollisionProfileName (Variables|Default|GetTriggerBox) "NoCollision" true :!class /Script/Engine.PrimitiveComponent)
  (Utilities|Time|SetTimerbyEvent (delegate Custom|EnableTriggerBox) 3e+01)
  (Default|CallRequestZombieSpawn (Math|Random|RandomIntegerinRange (Variables|Default|GetMinZombieSize) (Variables|Default|GetMaxZombieSize)) (Transformation|GetWorldLocation (Variables|Default|GetSpawnPoint))))

(event Custom|EnableTriggerBox
  (Collision|SetCollisionProfileName (Variables|Default|GetTriggerBox) "Trigger" true :!class /Script/Engine.PrimitiveComponent))

(event EventBeginPlay)

(event Collision|EventActorBeginOverlap
  (params (OtherActor :type Actor%20Object%20Reference)))

(event EventTick
  (params (DeltaSeconds :type Float%20%28single-precision%29)))

(fn ConstructionScript)