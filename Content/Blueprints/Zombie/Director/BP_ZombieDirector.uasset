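; Zombie director that tracks living zombies and serves spawn requests from spawners while capping the total at a maximum.
; On BeginPlay it registers every placed zombie and spawner and binds to their kill and spawn-request events.
; Requests spawn zombies at random reachable navmesh points near the requested location, registering each, and kills remove them from the list.
; Tick prints the remaining zombie count on screen for debugging.
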(event EventBeginPlay
  (Utilities|FlowControl|Sequence
    (:then_0
      (bind _outactors (Actor|GetAllActorsOfClass "/Game/Blueprints/Zombie/BP_Zombie.BP_Zombie_C"))
      (for _array_element _outactors
        (Private|RegisterZombieListener _array_element)))
    (:then_1
      (bind _outactors_2 (Actor|GetAllActorsOfClass "/Game/Blueprints/Zombie/Director/BP_ZombieSpawner.BP_ZombieSpawner_C"))
      (for _array_element_2 _outactors_2
        (Private|RegisterSpawnerListener _array_element_2)))))

(event EventTick
  (params (DeltaSeconds :type Float%20%28single-precision%29))
  (Development|PrintString (Utilities|String|Append "Zombie Left: " (Utilities|String|ToString(Integer) (Utilities|Array|Length (Variables|Default|GetZombies)))) true false "(R=0.000000,G=0.660000,B=1.000000,A=1.000000)" 0.01))

(fn ConstructionScript)

(fn RegisterZombieListener
  (params (Zombie :type BP%20Zombie%20Object%20Reference))
  (Utilities|Array|Add (Variables|Default|GetZombies) Zombie)
  ;[1 1 1] Listen to OnKill Event
  (EventDispatchers|BindEventtoOnZombieKill Zombie (EventDispatchers|CreateEvent :!event OnZombieKill)))

(fn OnZombieKill
  (params (Zombie :type BP%20Zombie%20Object%20Reference))
  (Utilities|Array|RemoveItem (Variables|Default|GetZombies) Zombie))

(fn RegisterSpawnerListener
  (params (ZombieSpawner :type BP%20Zombie%20Spawner%20Object%20Reference))
  (Utilities|Array|Add (Variables|Default|GetZombieSpawners) ZombieSpawner)
  (EventDispatchers|BindEventtoRequestZombieSpawn ZombieSpawner (EventDispatchers|CreateEvent :!event OnRequestZombieSpawn)))

(fn OnRequestZombieSpawn
  (params (SpawnCount :type Integer) (SpawnLocation :type Vector))
  (for _index (range 1 (Math|Integer|Min(Integer) SpawnCount (- (Variables|Default|GetMaxZombies) (Utilities|Array|Length (Variables|Default|GetZombies)))))
    (bind _returnvalue (Game|SpawnActorfromClass "/Game/Blueprints/Zombie/BP_Zombie.BP_Zombie_C" (Math|Transform|MakeTransform (+ (.RandomLocation (AI|Navigation|GetRandomReachablePointinRadius SpawnLocation 2e+02 0 0)) "0, 0,88.000000") "0, 0, 0" "1,1,1") "AdjustIfPossibleButDontSpawnIfColliding" 0 0))
    (Utilities|IsValid _returnvalue
      (:Is%20Valid
        (Private|RegisterZombieListener _returnvalue)))))