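; Explosive barrel that loses HP when hit, exploding at zero or catching fire on a non-lethal hit and exploding after a short fuse.
; The one-shot explosion fractures the destructible mesh, fires a radial impulse, plays effects and camera shake, then destroys the actor after a delay.
; Blast damage comes from briefly enabling Sphere overlaps, which send hit messages to zombies, players and other hittable actors.
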(event OnComponentBeginOverlap(Sphere)
  (params (OverlappedComponent :type Primitive%20Component%20Object%20Reference) (OtherActor :type Actor%20Object%20Reference) (OtherComp :type Primitive%20Component%20Object%20Reference) (OtherBodyIndex :type Integer) (bFromSweep :type Boolean) (SweepResult :type Hit%20Result%20Structure%20%28by%20ref%29))
  (bind _sm_barrel01_dm (Variables|Default|GetSM_Barrel01_DM))
  (bind _returnvalue (Transformation|GetWorldLocation _sm_barrel01_dm))
  ;[1 1 1] Kill Zombie
  (Class|BIZombieDamage|OnZombieHit(Message) OtherActor _returnvalue "0, 0, 0" (Math|Float|Truncate (Variables|Default|GetDamage)))
  (Class|BIHittable|OnHit(Message) OtherActor)
  (Class|BIPlayerDamage|OnPlayerHit(Message) OtherActor (Variables|Default|GetDamage) _returnvalue))

(event Custom|Explode
  (bind _sm_barrel01_dm (Variables|Default|GetSM_Barrel01_DM))
  (bind _returnvalue (Transformation|GetWorldLocation _sm_barrel01_dm))
  ;[1 1 1] Make sure wont run if exploded
  (if (not (Variables|Default|GetExploded))
    ;[1 1 1] Explosion
    (Utilities|FlowControl|DoOnce false
      (:Completed
        (Effects|SpawnEmitteratLocation "/Game/Assets/Import/Realistic_Starter_VFX_Pack_Vol2/Particles/Explosion/P_Explosion_Big_A.P_Explosion_Big_A" _returnvalue "0, 0, 0" "4.000000,4.000000,4.000000")
        (Class|DestructibleComponent|ApplyRadiusDamage (Variables|Default|GetSM_Barrel01_DM) 1.0 _returnvalue 2e+02 1e+04 true)
        (Audio|PlaySoundatLocation "/Game/StarterContent/Audio/Explosion_Cue.Explosion_Cue" _returnvalue "0, 0, 0" 1.0 1.0 0.0 0 0 0)
        (Class|RadialForceComponent|FireImpulse (Variables|Default|GetRadialForce))
        (Collision|SetCollisionProfileName (Variables|Default|GetSphere) "OverlapAllDynamic" true :!class /Script/Engine.PrimitiveComponent)
        (Utilities|FlowControl|Delay 0.1)
        (Collision|SetCollisionProfileName (Variables|Default|GetSphere) "NoCollision" true :!class /Script/Engine.PrimitiveComponent)
        (Camera|PlayWorldCameraShake "/Game/Blueprints/Interactable/BP_ExplosiveShake.BP_ExplosiveShake_C" (Transformation|GetActorLocation) 0.0 5e+03)
        (Rendering|SetVisibility (Variables|Default|GetFire%20Particle) false false)
        (Variables|Default|SetExploded true)
        (Audio|Components|Audio|Stop (Variables|Default|GetFireLoopSound))
        (Utilities|FlowControl|Delay 5.0)
        (Actor|DestroyActor)))))

(event EventBeginPlay
  ;[1 1 1] No Collision when start
  (Collision|SetCollisionProfileName (Variables|Default|GetSphere) "NoCollision" true :!class /Script/Engine.PrimitiveComponent))

(event EventOnHit
  (bind _returnvalue (Transformation|GetActorLocation))
  (bind _output_get (Variables|Default|SetHP (- (Variables|Default|GetHP) 1)))
  (if (<= _output_get 0)
    (CallFunction|Explode)
    (else
      (Utilities|FlowControl|DoOnce false
        (:Completed
          (Rendering|SetVisibility (Variables|Default|GetFire%20Particle) true false)
          (Audio|PlaySoundatLocation "/Game/Assets/Audio/Environment/Lighting_Fire.Lighting_Fire" _returnvalue "0, 0, 0" 1.0 1.0 0.0 0 0 0)
          (bind _returnvalue_2 (Audio|SpawnSoundatLocation "/Game/Assets/Audio/Environment/Fire_loop_Cue.Fire_loop_Cue" _returnvalue "0, 0, 0" 1.0 1.0 0.0 0 0))
          (Variables|Default|SetFireLoopSound _returnvalue_2)
          (Utilities|FlowControl|Delay 5.0)
          (CallFunction|Explode))))))

(fn ConstructionScript)