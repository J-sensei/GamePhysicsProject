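; Spawner actor that places an explosive barrel at its SpawnPoint on BeginPlay and keeps a reference to it.
; When an actor that casts to BP_FirstPersonController enters the Trigger and that barrel is no longer valid, it spawns a replacement.
; After respawning, it turns off the Trigger's collision and uses a timer to re-enable it, creating a 30-second cooldown.
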(event OnComponentBeginOverlap(Trigger)
  (params (OverlappedComponent :type Primitive%20Component%20Object%20Reference) (OtherActor :type Actor%20Object%20Reference) (OtherComp :type Primitive%20Component%20Object%20Reference) (OtherBodyIndex :type Integer) (bFromSweep :type Boolean) (SweepResult :type Hit%20Result%20Structure%20%28by%20ref%29))
  (Utilities|Casting|CastToBP_FirstPersonController OtherActor)
  (Utilities|IsValid (Variables|Default|GetExplosiveBarrel)
    (:Is%20Not%20Valid
      (bind _returnvalue (Game|SpawnActorfromClass "/Game/Blueprints/Interactable/BP_ExplosiveBarrel.BP_ExplosiveBarrel_C" (Math|Transform|MakeTransform (Transformation|GetWorldLocation (Variables|Default|GetSpawn%20Point)) "0, 0, 0" "1,1,1") "Undefined" 0 0))
      (Variables|Default|SetExplosiveBarrel _returnvalue)
      (Collision|SetCollisionProfileName (Variables|Default|GetTrigger) "NoCollision" true :!class /Script/Engine.PrimitiveComponent)
      (Utilities|Time|SetTimerbyEvent (delegate Custom|Enable) 3e+01))))

(event Custom|Enable
  (Collision|SetCollisionProfileName (Variables|Default|GetTrigger) "Trigger" true :!class /Script/Engine.PrimitiveComponent))

(event EventBeginPlay
  (bind _returnvalue (Game|SpawnActorfromClass "/Game/Blueprints/Interactable/BP_ExplosiveBarrel.BP_ExplosiveBarrel_C" (Math|Transform|MakeTransform (Transformation|GetWorldLocation (Variables|Default|GetSpawn%20Point)) "0, 0, 0" "1,1,1") "Undefined" 0 0))
  (Variables|Default|SetExplosiveBarrel _returnvalue))

(fn ConstructionScript)