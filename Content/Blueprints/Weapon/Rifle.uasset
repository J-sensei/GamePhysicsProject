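; Rifle weapon Blueprint that configures an assault rifle on top of a parent weapon class.
; The construction script fills structs for weapon stats, arm and rifle montages, AK47 sounds, muzzle flash and bullet decal, then calls the parent's construction script.
; It adds no active event logic of its own, and an older per-variable stat setup remains unconnected as a deprecated approach.
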(event EventBeginPlay
  (|CallParentFunction) ; This node is disabled and will not be called.\nDrag off pins to build functionality.
)

(event Collision|EventActorBeginOverlap
  (params (OtherActor :type Actor%20Object%20Reference))
  (|CallParentFunction OtherActor) ; This node is disabled and will not be called.\nDrag off pins to build functionality.
)

(event EventTick
  (params (DeltaSeconds :type Float%20%28single-precision%29))
  (|CallParentFunction DeltaSeconds) ; This node is disabled and will not be called.\nDrag off pins to build functionality.
)

(fn ConstructionScript
  (Variables|Default|SetWeaponData (Utilities|Struct|MakeWeaponData 0 "NewEnumerator0" 0 30 2.0 5e+02 0.5 9e+01 45.0 true))
  (Variables|Default|SetWeaponAnimations (Utilities|Struct|MakeWeaponAnimations "/Game/Assets/Import/FPS_Arm/Animation/Rifle/Montage/Arm_Rifle_Fire_Montage.Arm_Rifle_Fire_Montage" "/Game/Assets/Import/FPS_Weapon/Rifle/Animation/Rifle_Fire_Montage.Rifle_Fire_Montage" "/Game/Assets/Import/FPS_Arm/Animation/Rifle/ADS/Arm_Rifle_FireADS_Montage.Arm_Rifle_FireADS_Montage" "/Game/Assets/Import/FPS_Arm/Animation/Rifle/Montage/Arm_Rifle_Reload_Montage.Arm_Rifle_Reload_Montage" "/Game/Assets/Import/FPS_Weapon/Rifle/Animation/Rifle_Reload_Montage.Rifle_Reload_Montage"))
  (Variables|Default|SetWeaponSFX (Utilities|Struct|MakeWeaponSFX "/Game/Assets/Audio/Rifle_Fire/Ak47_Fire_Cue.Ak47_Fire_Cue" "/Game/Assets/Audio/Empty.Empty" "/Game/Assets/Audio/Shell.Shell" "(Default_4_B4E9F4F44EE541B6642D10B054ECFF3F=None,Wood_9_8D511E714422CDDA56CA16BDCB9F7EAD=None,Grass_10_D83FE2034B1922DB647365B409278477=None,Metal_11_37899AF74230D02D62C918859BC03DBF=None,Stone_13_A8A16EE147DBD7FC46F1CF9FF66A1F70=None,Water_17_C1DA15A347E148C24416FDA1461331F6=None,Enemy_15_56F8B4D142A8BA710B6140B34F92403B=None)"))
  (Variables|Default|SetWeaponParticles (Utilities|Struct|MakeWeaponParticles "/Game/Assets/Import/MilitaryWeapDark/FX/P_AssaultRifle_MuzzleFlash.P_AssaultRifle_MuzzleFlash" "(Default_2_57D3B35D43485299AB29E9BEB9D3F1C6=None,Wood_4_F0FC2BF34FFA2C0E3CCE04995F22B405=None,Grass_6_71BF2AAF4C58B65461F0D0AA16AE6E7F=None,Metal_8_593BB95D4DA99AF3C1876DA2AF85E414=None,Stone_13_E641ABA34A2B639F797705ACA1EB2727=None,Water_15_5B72BAB34902DC1CEF34CAA478D89168=None,Enemy_11_C695E1264535556BF8C4A5A6C8E4F19E=None)" "/Game/Blueprints/Weapon/Bullet/BulletDecal.BulletDecal_C"))
  (|CallParentFunction))