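; Pistol weapon Blueprint that supplies the handgun's data and assets to its parent class.
; The Construction Script fills structs for weapon stats, arm and weapon animations, per-surface sounds and particles, and projectile and shell references, then calls the parent script.
; The Event Graph holds only disabled events, and an older per-variable setup remains unconnected as deprecated.
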(event EventBeginPlay
  (|CallParentFunction) ; This node is disabled and will not be called.\nDrag off pins to build functionality.
)

(event Collision|EventActorBeginOverlap
  (params (OtherActor :type Actor%20Object%20Reference))
  (|CallParentFunction OtherActor) ; This node is disabled and will not be called.\nDrag off pins to build functionality.
)

(event EventTick
  (params (DeltaSeconds :type Float%20%28single-precision%29))
  (|CallParentFunction DeltaSeconds) ; This node is disabled and will not be called.\nDrag off pins to build functionality.
)

(fn ConstructionScript
  (Variables|Default|SetWeaponData (Utilities|Struct|MakeWeaponData "Pistol_C" "NewEnumerator1" 0 12 1.8 5e+02 0.1 9e+01 45.0 false false "PistolSocket" 0.5 "/Game/Assets/UI/GunIcon/handgun_icon_1.handgun_icon_1"))
  (Variables|Default|SetWeaponAnimations (Utilities|Struct|MakeWeaponAnimations "/Game/Assets/Import/FPS_Arm/Animation/Pistol/Arm_Pistol_Fire_Montage.Arm_Pistol_Fire_Montage" "/Game/Assets/Import/FPS_Weapon/Pistol/Animation/WeaponPistol_Fire_Montage.WeaponPistol_Fire_Montage" "/Game/Assets/Import/FPS_Arm/Animation/Pistol/ADS/Arm_Pistol_FireADS_Montage.Arm_Pistol_FireADS_Montage" "/Game/Assets/Import/FPS_Arm/Animation/Pistol/Arm_Pistol_Reload_Montage.Arm_Pistol_Reload_Montage" "/Game/Assets/Import/FPS_Weapon/Pistol/Animation/WeaponPistol_Reload_Montage.WeaponPistol_Reload_Montage"))
  (Variables|Default|SetWeaponSFX (Utilities|Struct|MakeWeaponSFX "/Game/Assets/Import/MilitaryWeapDark/Sound/Pistol/PistolB_Fire_Cue.PistolB_Fire_Cue" "/Game/Assets/Audio/Empty.Empty" "/Game/Assets/Audio/Shell.Shell" (Utilities|Struct|MakeImpactSFXTypes "/Game/Assets/Audio/BulletImpact/Stone/Stone_Impact_Cue.Stone_Impact_Cue" "/Game/Assets/Audio/BulletImpact/Wood.Wood" "/Game/Assets/Audio/BulletImpact/Grass.Grass" "/Game/Assets/Audio/BulletImpact/Metal.Metal" "/Game/Assets/Audio/BulletImpact/Stone/Stone_Impact_Cue.Stone_Impact_Cue" "/Game/Assets/Audio/BulletImpact/Stone/Stone_Impact_Cue.Stone_Impact_Cue" "/Game/Assets/Import/MilitaryWeapDark/Sound/Rifle/Rifle_ImpactBody_Cue.Rifle_ImpactBody_Cue") "/Game/Assets/Import/MilitaryWeapDark/Sound/Pistol/Pistol_ReloadEject_Cue.Pistol_ReloadEject_Cue" "/Game/Assets/Import/MilitaryWeapDark/Sound/Pistol/Wavs/Pistol_ReloadMagInsert01.Pistol_ReloadMagInsert01" "/Game/Assets/Import/MilitaryWeapDark/Sound/Pistol/Pistol_ReloadInsert_Cue.Pistol_ReloadInsert_Cue"))
  (Variables|Default|SetWeaponParticles (Utilities|Struct|MakeWeaponParticles "/Game/Assets/Import/MilitaryWeapDark/FX/P_Pistol_MuzzleFlash_01.P_Pistol_MuzzleFlash_01" (Utilities|Struct|MakeImpactParticleTypes "/Game/Assets/Import/MilitaryWeapDark/FX/P_Impact_Stone_Medium_01.P_Impact_Stone_Medium_01" "/Game/Assets/Import/MilitaryWeapDark/FX/P_Impact_Wood_Medium_01.P_Impact_Wood_Medium_01" "/Game/Assets/Import/MilitaryWeapDark/FX/P_Impact_Stone_Medium_01.P_Impact_Stone_Medium_01" "/Game/Assets/Import/MilitaryWeapDark/FX/P_Impact_Metal_Medium_01.P_Impact_Metal_Medium_01" "/Game/Assets/Import/MilitaryWeapDark/FX/P_Impact_Stone_Medium_01.P_Impact_Stone_Medium_01" "/Game/Assets/Import/MilitaryWeapDark/FX/P_Impact_Stone_Medium_01.P_Impact_Stone_Medium_01" "/Game/Assets/Import/Realistic_Starter_VFX_Pack_Vol2/Particles/Blood/P_Blood_Splat_Cone.P_Blood_Splat_Cone") "/Game/Blueprints/Weapon/Bullet/BulletDecal.BulletDecal_C" "/Game/Blueprints/Weapon/Bullet/PistolProjectile.PistolProjectile_C" "/Game/Blueprints/Weapon/Shell/PistolShell.PistolShell_C"))
  (|CallParentFunction))