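; Base weapon Blueprint that handles firing, reloading and aim-down-sights by delegating the work to a WeaponComponent.
; The construction script unpacks data, animation, SFX and particle structs into variables and fills the magazine.
; Shoot checks ammo, then has the component update ammo, raycast with spread and apply muzzle flash, decal, shell and recoil, or play an empty sound.
; The local Reload graph is unused, as OnReload calls the component instead.
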(event Custom|OnReload
  ;[1 1 1] Reload Events
  (if (< (Variables|Data|GetCurrentAmmo) (Variables|Data|GetMaxAmmo))
    (Default|ReloadBegin (Variables|Default|GetWeaponComponent) (Variables|Default|GetWeaponBase) (Variables|Data|GetReloadTime))))

(event Custom|OnFire
  ;[1 1 1] Call the shoot function
  (CallFunction|Shoot))

(event Custom|OnADS
  (params (Alpha :type Float%20%28single-precision%29))
  ;[1 1 1] Call ADS Begin in Weapon Component
  (Default|ADSBegin (Variables|Default|GetWeaponComponent) (Variables|Default|GetScope) Alpha (Variables|Data|GetFieldOfView) (Variables|Data|GetCameraDistance)))

(event EventBeginPlay)

(event Collision|EventActorBeginOverlap
  (params (OtherActor :type Actor%20Object%20Reference)))

(event EventTick
  (params (DeltaSeconds :type Float%20%28single-precision%29)))

(fn ConstructionScript
  (bind _weaponparticles (Variables|Structure|GetWeaponParticles))
  (bind _weaponsfx (Variables|Structure|GetWeaponSFX))
  (bind _weaponanimations (Variables|Structure|GetWeaponAnimations))
  (Utilities|FlowControl|Sequence
    (:then_0
      ;[1 1 1] Set Weapon Data
      (Variables|Structure|SetWeaponData (Utilities|Struct|MakeWeaponData (Utilities|GetClass self) (.name (Variables|Structure|GetWeaponData)) (.currentammo (Variables|Structure|GetWeaponData)) (.maxammo (Variables|Structure|GetWeaponData)) (.reloadtime (Variables|Structure|GetWeaponData)) (.spread (Variables|Structure|GetWeaponData)) (.recoil (Variables|Structure|GetWeaponData)) (.fieldofview (Variables|Structure|GetWeaponData)) (.cameradistance (Variables|Structure|GetWeaponData)) (.firemode (Variables|Structure|GetWeaponData))))
      (bind _output_get (Variables|Data|SetMaxAmmo (.maxammo (Variables|Structure|GetWeaponData))))
      (Variables|Data|SetCurrentAmmo _output_get)
      (Variables|Data|SetReloadTime (.reloadtime (Variables|Structure|GetWeaponData)))
      (Variables|Data|SetFireMode (.firemode (Variables|Structure|GetWeaponData)))
      (Variables|Data|SetSpread (.spread (Variables|Structure|GetWeaponData)))
      (Variables|Data|SetRecoil (.recoil (Variables|Structure|GetWeaponData)))
      ;;[1 1 1] Set ADS Field of View
      (Variables|Data|SetFieldOfView (.fieldofview (Variables|Structure|GetWeaponData)))
      (Variables|Data|SetCameraDistance (.cameradistance (Variables|Structure|GetWeaponData))))
    (:then_1
      ;[1 1 1] Set Weapon Animations
      (Variables|Animation|SetArmFireAnim (.armfire _weaponanimations))
      (Variables|Animation|SetWeaponFireAnim (.weaponfire _weaponanimations))
      (Variables|Animation|SetArmADSFireAnim (.armadsfire _weaponanimations))
      (Variables|Animation|SetArmReloadAnim (.armreload _weaponanimations))
      (Variables|Animation|SetWeaponReloadAnim (.weaponreload _weaponanimations)))
    (:then_2
      ;[1 1 1] Set Weapon SFXs
      (Variables|SFX|SetFireSFX (.fire _weaponsfx))
      (Variables|SFX|SetEmptySFX (.empty _weaponsfx))
      (Variables|SFX|SetShellSFX (.shell _weaponsfx)))
    (:then_3
      ;[1 1 1] Set Weapon Particles
      (Variables|Particle|SetMuzzleParticle (.muzzle _weaponparticles))
      (Variables|Particle|SetDecal (.decal _weaponparticles)))))

(fn Shoot
  ;[1 1 1] Check Ammo
  (if (> (Variables|Data|GetCurrentAmmo) 0)
    ;[1 1 1] Calculate shoot vector
    (Default|UpdateAmmo (Variables|Default|GetWeaponComponent) (Variables|Default|GetWeaponBase) (Variables|Data|GetCurrentAmmo) (Variables|Animation|GetWeaponFireAnim))
    (bind (_hitlocation _hitnormal _hitactor) (Default|GunRaycast (Variables|Default|GetWeaponComponent) (Variables|Default|GetMuzzle) (Variables|Data|GetSpread)))
    (Utilities|FlowControl|Sequence
      (:then_0
        ;[0.2254 0.3783 1] Polish the gun shoot feedbacks
        (Default|MuzzleFlashParticle (Variables|Default|GetWeaponComponent) (Variables|Default|GetMuzzle) (Variables|Particle|GetMuzzleParticle)))
      (:then_1
        (Default|SpawnDecal (Variables|Default|GetWeaponComponent) _hitlocation _hitnormal (Variables|Particle|GetDecal)))
      (:then_2
        (Default|SpawnShell (Variables|Default|GetWeaponComponent) (Variables|Default|GetWeaponBase) "/Game/Blueprints/Weapon/Shell/Shell.Shell_C"))
      (:then_3
        (Default|Recoil (Variables|Default|GetWeaponComponent) (Variables|Data|GetRecoil)))
      (:then_4
        ;;[1 1 1] Events Trigger when fire
        (Default|FireBegin (Variables|Default|GetWeaponComponent)))
      (:then_5
        (Development|PrintString (Utilities|String|Append "Hit: " (Utilities|GetObjectName _hitactor)))))
    (else
      (Default|EmptySFX (Variables|Default|GetWeaponComponent)))))