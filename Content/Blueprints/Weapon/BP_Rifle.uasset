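; BP_Rifle is a data-only style rifle weapon Blueprint that configures a parent weapon class.
; Its construction script fills structs for weapon stats, fire and reload montages, sounds and particle, decal, projectile and shell references, then calls the parent construction script.
; The event graph holds only disabled stubs, and an unconnected older set of per-variable assignments remains as deprecated setup.
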(event EventBeginPlay
  (|CallParentFunction) ; This node is disabled and will not be called.\nDrag off pins to build functionality.
)

(event Collision|EventActorBeginOverlap
  (params (OtherActor :type Actor%20Object%20Reference))
  (|CallParentFunction OtherActor) ; This node is disabled and will not be called.\nDrag off pins to build functionality.
)

(event EventTick
  (params (DeltaSeconds :type Float%20%28single-precision%29))
  (|CallParentFunction DeltaSeconds) ; This node is disabled and will not be called.\nDrag off pins to build functionality.
)

(fn ConstructionScript
  (Variables|Default|SetWeaponData (Utilities|Struct|MakeF_WeaponData "BP_Rifle_C" "NewEnumerator0" 0 30 0 2.0 5e+03 0.8 9e+01 45.0 true true "RifleSocket" 0.1 "/Game/Assets/UI/Icon/Rifle.Rifle"))
  (Variables|Default|SetWeaponAnimations (Utilities|Struct|MakeF_WeaponAnimations "/Game/Assets/Import/FPS_Arm/Animation/Rifle/Montage/Arm_Rifle_Fire_Montage.Arm_Rifle_Fire_Montage" "/Game/Assets/Import/FPS_Weapon/Rifle/Animation/Rifle_Fire_Montage.Rifle_Fire_Montage" "/Game/Assets/Import/FPS_Arm/Animation/Rifle/ADS/Arm_Rifle_FireADS_Montage.Arm_Rifle_FireADS_Montage" "/Game/Assets/Import/FPS_Arm/Animation/Rifle/Montage/Arm_Rifle_Reload_Montage.Arm_Rifle_Reload_Montage" "/Game/Assets/Import/FPS_Weapon/Rifle/Animation/Rifle_Reload_Montage.Rifle_Reload_Montage"))
  (Variables|Default|SetWeaponSFX (Utilities|Struct|MakeF_WeaponSFX "/Game/Assets/Audio/Rifle_Fire/Ak47_Fire_Cue.Ak47_Fire_Cue" "/Game/Assets/Audio/Empty.Empty" "/Game/Assets/Audio/Shell.Shell" (Utilities|Struct|MakeF_ImpactSFXTypes "/Game/Assets/Import/MilitaryWeapDark/Sound/Rifle/Rifle_ImpactSurface_Cue.Rifle_ImpactSurface_Cue" "/Game/Assets/Audio/BulletImpact/Wood.Wood" "/Game/Assets/Audio/BulletImpact/Grass.Grass" "/Game/Assets/Audio/BulletImpact/Metal.Metal" "/Game/Assets/Audio/BulletImpact/Stone/Stone_Impact_Cue.Stone_Impact_Cue" "/Game/Assets/Audio/BulletImpact/Stone/Stone_Impact_Cue.Stone_Impact_Cue" "/Game/Assets/Import/MilitaryWeapDark/Sound/Rifle/Rifle_ImpactBody_Cue.Rifle_ImpactBody_Cue") "/Game/Assets/Audio/Reload_Eject.Reload_Eject" "/Game/Assets/Audio/Reload_Insert.Reload_Insert" "/Game/Assets/Audio/Reload_Load.Reload_Load"))
  (Variables|Default|SetWeaponParticles (Utilities|Struct|MakeF_WeaponParticles "/Game/Assets/Import/MilitaryWeapDark/FX/P_AssaultRifle_MuzzleFlash.P_AssaultRifle_MuzzleFlash" (Utilities|Struct|MakeF_ImpactParticleTypes "/Game/Assets/Import/MilitaryWeapDark/FX/P_Impact_Stone_Large_01.P_Impact_Stone_Large_01" "/Game/Assets/Import/MilitaryWeapDark/FX/P_Impact_Wood_Large_01.P_Impact_Wood_Large_01" "/Game/Assets/Import/MilitaryWeapDark/FX/P_Impact_Stone_Large_01.P_Impact_Stone_Large_01" "/Game/Assets/Import/MilitaryWeapDark/FX/P_Impact_Metal_Large_01.P_Impact_Metal_Large_01" "/Game/Assets/Import/MilitaryWeapDark/FX/P_Impact_Stone_Large_01.P_Impact_Stone_Large_01" "/Game/Assets/Import/MilitaryWeapDark/FX/P_Impact_Stone_Large_01.P_Impact_Stone_Large_01" "/Game/Assets/Import/Realistic_Starter_VFX_Pack_Vol2/Particles/Blood/P_Blood_Splat_Cone.P_Blood_Splat_Cone") "/Game/Blueprints/Weapon/Bullet/BP_BulletDecal.BP_BulletDecal_C" "/Game/Blueprints/Weapon/Bullet/BP_Projectile.BP_Projectile_C" "/Game/Blueprints/Weapon/Shell/BP_Shell.BP_Shell_C"))
  (|CallParentFunction))