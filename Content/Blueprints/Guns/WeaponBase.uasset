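; Base gun Blueprint that handles firing, reloading and aim-down-sights, delegating most of the work to a WeaponComponent.
; Shoot checks ammo, then has the component update ammo, raycast with spread, and drive muzzle flash, decal, shell, recoil and fire events, or play empty SFX.
; OnReload refills ammo immediately before calling ReloadBegin, and OnADS passes scope and camera settings to ADSBegin.
; The delayed Reload graph is unused, and hits only print the actor name.
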(event Custom|OnReload
  ;[1 1 1] Reload Events
  (if (< (Variables|Default|GetCurrentAmmo) (Variables|Default|GetMaxAmmo))
    (Variables|Default|SetCurrentAmmo (Variables|Default|GetMaxAmmo))
    (Default|ReloadBegin (Variables|Default|GetWeaponComponent) (Variables|Default|GetWeaponBase) (Variables|Default|GetReloadTime))))

(event Custom|OnFire
  ;[1 1 1] Call the shoot function
  (CallFunction|Shoot))

(event Custom|OnADS
  (params (Alpha :type Float%20%28single-precision%29))
  ;[1 1 1] Call ADS Begin in Weapon Component
  (Default|ADSBegin (Variables|Default|GetWeaponComponent) (Variables|Default|GetScope) Alpha (Variables|Default|GetFieldOfView) (Variables|Default|GetCameraDistance)))

(event EventBeginPlay)

(event Collision|EventActorBeginOverlap
  (params (OtherActor :type Actor%20Object%20Reference)))

(event EventTick
  (params (DeltaSeconds :type Float%20%28single-precision%29)))

(fn ConstructionScript)

(fn Shoot
  ;[1 1 1] Check Ammo
  (if (> (Variables|Default|GetCurrentAmmo) 0)
    ;[1 1 1] Calculate shoot vector
    (Default|UpdateAmmo (Variables|Default|GetWeaponComponent) (Variables|Default|GetWeaponBase) (Variables|Default|GetCurrentAmmo) "/Game/Assets/Import/FPS_Weapon/Rifle/Animation/Rifle_Fire.Rifle_Fire")
    (bind (_hitlocation _hitnormal _hitactor) (Default|GunRaycast (Variables|Default|GetWeaponComponent) (Variables|Default|GetMuzzle) (Variables|Default|GetSpread)))
    (Utilities|FlowControl|Sequence
      (:then_0
        ;[0.2254 0.3783 1] Polish the gun shoot feedbacks
        (Default|MuzzleFlashParticle (Variables|Default|GetWeaponComponent) (Variables|Default|GetMuzzle) "/Game/Assets/Import/MilitaryWeapDark/FX/P_AssaultRifle_MuzzleFlash.P_AssaultRifle_MuzzleFlash"))
      (:then_1
        (Default|SpawnDecal (Variables|Default|GetWeaponComponent) _hitlocation _hitnormal "/Game/Blueprints/Guns/Bullet/BulletDecal.BulletDecal_C"))
      (:then_2
        (Default|SpawnShell (Variables|Default|GetWeaponComponent) (Variables|Default|GetWeaponBase) "/Game/Blueprints/Guns/Shell/Shell.Shell_C"))
      (:then_3
        (Default|Recoil (Variables|Default|GetWeaponComponent) (Variables|Default|GetRecoil)))
      (:then_4
        ;;[1 1 1] Events Trigger when fire
        (Default|FireBegin (Variables|Default|GetWeaponComponent)))
      (:then_5
        (Development|PrintString (Utilities|String|Append "Hit: " (Utilities|GetObjectName _hitactor)))))
    (else
      (Default|EmptySFX (Variables|Default|GetWeaponComponent)))))