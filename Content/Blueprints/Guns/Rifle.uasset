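; Rifle gun Blueprint that sets up the weapon's stats.
; Its construction script runs the parent setup, then assigns starting and maximum ammo, reload time, fire mode, spread and recoil.
; The event graph holds only disabled default events, so this Blueprint adds no behavior of its own beyond those values.
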(event EventBeginPlay
  (|CallParentFunction) ; This node is disabled and will not be called.\nDrag off pins to build functionality.
)

(event Collision|EventActorBeginOverlap
  (params (OtherActor :type Actor%20Object%20Reference))
  (|CallParentFunction OtherActor) ; This node is disabled and will not be called.\nDrag off pins to build functionality.
)

(event EventTick
  (params (DeltaSeconds :type Float%20%28single-precision%29))
  (|CallParentFunction DeltaSeconds) ; This node is disabled and will not be called.\nDrag off pins to build functionality.
)

(fn ConstructionScript
  (|CallParentFunction)
  (bind _output_get (Variables|Default|SetCurrentAmmo 15))
  (Variables|Default|SetMaxAmmo _output_get)
  (Variables|Default|SetReloadTime 2.0)
  (Variables|Default|SetFireMode true)
  (Variables|Default|SetSpread 5e+02)
  (Variables|Default|SetRecoil 0.5))