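; Base pickup Actor that drops to the surface beneath it on BeginPlay via a downward line trace and destroys itself after a short lifetime.
; When a BP_FirstPersonController overlaps its Box, it calls OnPickup, plays the pickup particle and sound, then destroys itself.
; OnPickup is empty here, acting as the hook for the pickup's actual effect.
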(event OnComponentBeginOverlap(Box)
  (params (OverlappedComponent :type Primitive%20Component%20Object%20Reference) (OtherActor :type Actor%20Object%20Reference) (OtherComp :type Primitive%20Component%20Object%20Reference) (OtherBodyIndex :type Integer) (bFromSweep :type Boolean) (SweepResult :type Hit%20Result%20Structure%20%28by%20ref%29))
  (bind _returnvalue (Transformation|GetActorLocation))
  (bind _asbp_first_person_controller (Utilities|Casting|CastToBP_FirstPersonController OtherActor))
  (CallFunction|OnPickup _asbp_first_person_controller)
  (Niagara|SpawnSystematLocation (Variables|Default|GetPickupParticle) _returnvalue "0, 0, 0" "4.000000,4.000000,4.000000")
  (Audio|PlaySoundatLocation (Variables|Default|GetPickupSound) _returnvalue "0, 0, 0" 1.0 1.0 0.0 0 0 0)
  (Actor|DestroyActor))

(event Custom|OnPickup
  (params (FirstPersonController :type BP%20First%20Person%20Controller%20Object%20Reference)))

(event EventBeginPlay
  (bind _outhit (Collision|LineTraceByChannel (Transformation|GetActorLocation) (+ (Transformation|GetActorLocation) (* (Math|Vector|VectorDown) 5e+02)) "TraceTypeQuery1" false 0 "None"))
  (Transformation|SetWorldLocationAndRotation (Variables|Default|GetDefaultSceneRoot) (.Location (Collision|BreakHitResult _outhit)) "0, 0, 0" false false)
  (Utilities|FlowControl|Delay 1e+01)
  (Actor|DestroyActor))

(fn ConstructionScript)